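; BP_Target_PlusTime is a target actor that grants bonus time when shot.
; When a FirstPersonProjectile begins overlapping its TargetCollision component, it casts the game mode to BP_GameModeGamePlay and adds BonusTime to GameTimeLimit.
; The actor does not destroy itself or the projectile in this graph, and its BeginPlay, Tick and actor overlap events are disabled stubs.
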(event OnComponentBeginOverlap(TargetCollision)
  (params (OverlappedComponent :type Primitive%20Component%20Object%20Reference) (OtherActor :type Actor%20Object%20Reference) (OtherComp :type Primitive%20Component%20Object%20Reference) (OtherBodyIndex :type Integer) (bFromSweep :type Boolean) (SweepResult :type Hit%20Result%20Structure%20%28by%20ref%29))
  ;[1 1 1] Add Time to play
  (Utilities|Casting|CastToFirstPersonProjectile OtherActor)
  (bind _asbp_game_mode_game_play (Utilities|Casting|CastToBP_GameModeGamePlay (Game|GetGameMode)))
  (Variables|/Game/1St_Folder/Blueprints/Framework/BP_GameModeGamePlay.BP_GameModeGamePlay_C|SetGameTimeLimit _asbp_game_mode_game_play (+ (Variables|/Game/1St_Folder/Blueprints/Framework/BP_GameModeGamePlay.BP_GameModeGamePlay_C|GetGameTimeLimit _asbp_game_mode_game_play) (Variables|Default|GetBonusTime))))

(event EventBeginPlay
  (|CallParentFunction) ; This node is disabled and will not be called.\nDrag off pins to build functionality.
)

(event Collision|EventActorBeginOverlap
  (params (OtherActor :type Actor%20Object%20Reference))
  (|CallParentFunction OtherActor) ; This node is disabled and will not be called.\nDrag off pins to build functionality.
)

(event EventTick
  (params (DeltaSeconds :type Float%20%28single-precision%29))
  (|CallParentFunction DeltaSeconds) ; This node is disabled and will not be called.\nDrag off pins to build functionality.
)

(fn ConstructionScript
  (|CallParentFunction))