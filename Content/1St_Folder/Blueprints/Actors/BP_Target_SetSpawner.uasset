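; Trigger actor that spawns a set of five targets when the first-person player enters its volume.
; The overlap event casts to FirstPersonCharacter and passes a DoOnce, so the set spawns only once.
; A Sequence starts five parallel delays, each spawning its own target class at its matching spawn component's transform after a per-target delay.
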(event OnComponentBeginOverlap(TriggerVolume)
  (params (OverlappedComponent :type Primitive%20Component%20Object%20Reference) (OtherActor :type Actor%20Object%20Reference) (OtherComp :type Primitive%20Component%20Object%20Reference) (OtherBodyIndex :type Integer) (bFromSweep :type Boolean) (SweepResult :type Hit%20Result%20Structure%20%28by%20ref%29))
  (Utilities|Casting|CastToFirstPersonCharacter OtherActor)
  (Utilities|FlowControl|DoOnce false
    (:Completed
      (Utilities|FlowControl|Sequence
        (:then_0
          ;[1 1 1] Target_01
          (Utilities|FlowControl|Delay (Variables|Default|Gettarget_01_delay))
          (Game|SpawnActorfromClass (Variables|Default|Gettarget_01) (Transformation|GetWorldTransform (Variables|Default|GetSpawnTarget_01)) "Undefined" 0 0))
        (:then_1
          ;[1 1 1] Target_02
          (Utilities|FlowControl|Delay (Variables|Default|Gettarget_02_delay))
          (Game|SpawnActorfromClass (Variables|Default|Gettarget_02) (Transformation|GetWorldTransform (Variables|Default|GetSpawnTarget_02)) "Undefined" 0 0))
        (:then_2
          ;[1 1 1] Target_03
          (Utilities|FlowControl|Delay (Variables|Default|Gettarget_03_delay))
          (Game|SpawnActorfromClass (Variables|Default|Gettarget_03) (Transformation|GetWorldTransform (Variables|Default|GetSpawnTarget_03)) "Undefined" 0 0))
        (:then_3
          ;[1 1 1] Target_04
          (Utilities|FlowControl|Delay (Variables|Default|Gettarget_04_delay))
          (Game|SpawnActorfromClass (Variables|Default|Gettarget_04) (Transformation|GetWorldTransform (Variables|Default|GetSpawnTarget_04)) "Undefined" 0 0))
        (:then_4
          ;[1 1 1] Target_05
          (Utilities|FlowControl|Delay (Variables|Default|Gettarget_05_delay))
          (Game|SpawnActorfromClass (Variables|Default|Gettarget_05) (Transformation|GetWorldTransform (Variables|Default|GetSpawnTarget_05)) "Undefined" 0 0))))))

(fn ConstructionScript)