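; BP_Door is an interactable door actor that the player opens once by pressing F.
; When a FirstPersonCharacter overlaps the Collision component, it shows a TextRender prompt and allows opening, unless the door has already been opened.
; Pressing F hides the prompt, flags the door as opened and plays the DoorOpen timeline, which drives the Door's relative yaw.
; Leaving the overlap hides the prompt and disables opening.
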(event OnComponentBeginOverlap(Collision)
  (params (OverlappedComponent :type Primitive%20Component%20Object%20Reference) (OtherActor :type Actor%20Object%20Reference) (OtherComp :type Primitive%20Component%20Object%20Reference) (OtherBodyIndex :type Integer) (bFromSweep :type Boolean) (SweepResult :type Hit%20Result%20Structure%20%28by%20ref%29))
  ;[1 1 1] Show/Hide Open door message
  (Utilities|Casting|CastToFirstPersonCharacter OtherActor)
  (if (not (Variables|Default|GethasDoorBeenOpened))
    (Rendering|SetVisibility (Variables|Default|GetTextRender) true false)
    (Variables|Default|SetcanOpenDoor true)))

(event OnComponentEndOverlap(Collision)
  (params (OverlappedComponent :type Primitive%20Component%20Object%20Reference) (OtherActor :type Actor%20Object%20Reference) (OtherComp :type Primitive%20Component%20Object%20Reference) (OtherBodyIndex :type Integer))
  ;[1 1 1] Show/Hide Open door message
  (Utilities|Casting|CastToFirstPersonCharacter OtherActor)
  (Rendering|SetVisibility (Variables|Default|GetTextRender) false false)
  (Variables|Default|SetcanOpenDoor false))

(event Input|KeyboardEvents|F
  (params (Key :type Key%20Structure :default "None"))
  ;[1 1 1] Open Door
  (:Pressed
    (if (Variables|Default|GetcanOpenDoor)
      (Rendering|SetVisibility (Variables|Default|GetTextRender) false false)
      (Variables|Default|SethasDoorBeenOpened true)
      (bind _doorrotation (Timeline|DoorOpen Play)
        (:Update
          (Transformation|SetRelativeRotation (Variables|Default|GetDoor) (Math|Rotator|MakeRotator 0.0 0.0 _doorrotation) false false))))))

(fn ConstructionScript)