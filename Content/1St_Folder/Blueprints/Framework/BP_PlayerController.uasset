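; Player controller Blueprint that toggles a pause menu when the P key is pressed.
; An IsGamePaused flag selects between creating the menu widget and removing it from the viewport.
; Each toggle also sets the game's paused state, cursor visibility and input mode, using Game and UI with widget focus while paused and Game Only otherwise.
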(event Input|KeyboardEvents|P
  (params (Key :type Key%20Structure :default "None"))
  (bind _self self)
  ;[1 1 1] Paused Game with "P" key
  (:Pressed
    (if (Variables|Default|GetisGamePaused)
      (Variables|Default|SetisGamePaused false)
      (Widget|RemovefromParent (stale _returnvalue))
      (Variables|Default|SetbShowMouseCursor false)
      (Input|SetInputModeGameOnly _self)
      (Game|SetGamePaused false)
      (else
        (Variables|Default|SetisGamePaused true)
        (bind _returnvalue (UserInterface|CreateWidget "/Game/1St_Folder/UI/WBP_PauseMenu.WBP_PauseMenu_C"))
        (UserInterface|Viewport|AddtoViewport _returnvalue 0)
        (Variables|Default|SetbShowMouseCursor true)
        (Input|SetInputModeGameandUI _self _returnvalue "DoNotLock" true)
        (Game|SetGamePaused true)))))

(fn ConstructionScript)