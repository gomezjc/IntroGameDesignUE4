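; Gameplay game mode that runs a level's HUD, music, countdown, points and player respawning.
; BeginPlay picks the time limit from the game instance's selected level and starts a one-second looping timer that triggers game over at zero.
; A destroyed player is respawned at RespawnTransform after a delay, possessed, then rebound to the destroy event.
; Level-finish and game-over events pause the timer, switch to UI input, show their menu and swap music.
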(event Custom|OnDestroyed_Event_0
  (params (DestroyedActor :type Actor%20Object%20Reference))
  ;[1 1 1] Respawn Player
  (Utilities|FlowControl|Delay 2.0)
  (bind _returnvalue (Game|SpawnActorfromClass "/Game/FirstPersonBP/Blueprints/FirstPersonCharacter.FirstPersonCharacter_C" (Variables|Default|GetrespawnTransform) "Undefined" (stale Custom|Respawn _asfirst_person_character) 0))
  (Pawn|Possess (Game|GetPlayerController 0) _returnvalue)
  (CallFunction|Respawn))

(event Custom|LevelFinish
  (bind _returnvalue (Game|GetPlayerController 0))
  ;[1 1 1] Level complete
  (Utilities|Time|PauseTimerbyHandle (Variables|Default|GetTimer))
  (Input|DisableInput (Game|GetPlayerCharacter 0) _returnvalue)
  (Input|SetInputModeUIOnly _returnvalue 0 "DoNotLock")
  (Variables|/Script/Engine.PlayerController|SetbShowMouseCursor _returnvalue true)
  (bind _returnvalue_2 (UserInterface|CreateWidget "/Game/1St_Folder/UI/WBP_LevelComplete.WBP_LevelComplete_C"))
  (UserInterface|Viewport|AddtoViewport _returnvalue_2 0)
  (Audio|Components|Audio|FadeOut (Variables|Default|GetMusicGame) 0.5 0.0 :!class /Script/Engine.AudioComponent)
  (Audio|Components|Audio|Play (Variables|Default|GetMusicLevelComplete) 0.0))

(event Custom|Respawn
  ;[1 1 1] Respawn Player
  (bind _asfirst_person_character (Utilities|Casting|CastToFirstPersonCharacter (Game|GetPlayerCharacter 0)))
  (Game|AssignOnDestroyed _asfirst_person_character (delegate Custom|OnDestroyed_Event_0)))

(event Custom|GameOverEvent
  (bind _returnvalue (Game|GetPlayerController 0))
  ;[1 1 1] GameOver
  (Utilities|Time|PauseTimerbyHandle (Variables|Default|GetTimer))
  (Input|DisableInput (Game|GetPlayerCharacter 0) _returnvalue)
  (Input|SetInputModeUIOnly _returnvalue 0 "DoNotLock")
  (Variables|/Script/Engine.PlayerController|SetbShowMouseCursor _returnvalue true)
  (bind _returnvalue_2 (UserInterface|CreateWidget "/Game/1St_Folder/UI/WBP_GameOverMenu.WBP_GameOverMenu_C"))
  (UserInterface|Viewport|AddtoViewport _returnvalue_2 0)
  (Audio|Components|Audio|FadeOut (Variables|Default|GetMusicGame) 0.5 0.0 :!class /Script/Engine.AudioComponent)
  (Audio|Components|Audio|Play (Variables|Default|GetMusicGameOver) 0.0))

(event EventBeginPlay
  (Utilities|FlowControl|Sequence
    (:then_0
      ;[1 1 1] Show HUD
      (bind _returnvalue (UserInterface|CreateWidget "/Game/1St_Folder/UI/WBP_HUD.WBP_HUD_C"))
      (UserInterface|Viewport|AddtoViewport _returnvalue 0))
    (:then_1
      ;[1 1 1] Game Music
      (Audio|Components|Audio|Play (Variables|Default|GetMusicGame) 0.0))
    (:then_2
      ;[1 1 1] Set Game Time Limit base on level selected
      (bind _asbp_game_instance (Utilities|Casting|CastToBP_GameInstance (Game|GetGameInstance)))
      (Variables|Default|SetGameTimeLimit (Utilities|Select :Index (Variables|/Game/1St_Folder/Blueprints/Framework/BP_GameInstance.BP_GameInstance_C|GetLevelSelected _asbp_game_instance) :NewEnumerator0 (Variables|Default|GetLevel_01_Timelimit) :NewEnumerator1 (Variables|Default|GetLevel_02_Timelimit) :NewEnumerator2 (Variables|Default|GetLevel_03_Timelimit))))
    (:then_3
      ;[1 1 1] Timer
      (bind _returnvalue_2 (Utilities|Time|SetTimerbyFunctionName 0 "decrementTimer" 1.0 true))
      (Variables|Default|SetTimer _returnvalue_2))
    (:then_4
      ;[1 1 1] Respawn Player
      (bind _asfirst_person_character (Utilities|Casting|CastToFirstPersonCharacter (Game|GetPlayerCharacter 0)))
      (Game|AssignOnDestroyed _asfirst_person_character (delegate Custom|OnDestroyed_Event_0)))))

(fn ConstructionScript)

(fn AddPoints
  (params (PointToAdd :type Integer))
  (Variables|Default|SetGamePoints (+ PointToAdd (Variables|Default|GetGamePoints))))

(fn DecrementTimer
  (bind _output_get (Variables|Default|SetGameTimeLimit (- (Variables|Default|GetGameTimeLimit) 1)))
  (if (== _output_get 0)
    (CallFunction|GameOverEvent)))